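; BP_Player is the 2D Paper2D player character, adding the default Enhanced Input mapping context on BeginPlay.
; The movement input moves it along its forward vector, swaps run and idle flipbooks, and rotates the sprite 180 degrees to face travel direction.
; An IsJumping flag gates movement.
; Jump logic with a jump flipbook and delayed landing check exists but is unconnected, and never clears that flag.
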(event Input|EnhancedActionEvents|EnhancedInputActionIA_Movement
  (params (ActionValue :type Float%20%28double-precision%29) (ElapsedSeconds :type Float%20%28double-precision%29) (TriggeredSeconds :type Float%20%28double-precision%29) (InputAction :type Input%20Action%20Object%20Reference :default "/Game/Assets/Player/Blueprints/IA_Movement.IA_Movement"))
  (:Triggered
    (if (not (Variables|Default|GetisJumping))
      (Pawn|Input|AddMovementInput (Transformation|GetActorForwardVector) ActionValue false)
      (Sprite|SetFlipbook (Variables|Default|GetPaperFlipbook) "/Game/Assets/Player/Animations/Player_Run.Player_Run")
      (if (> ActionValue 0.0)
        (Transformation|SetWorldRotation (Variables|Default|GetPaperFlipbook) "0, 0, 0" false false)
        (else
          (Transformation|SetWorldRotation (Variables|Default|GetPaperFlipbook) "0.000000,-180.000000,0.000000" false false)))))
  (:Completed
    (if (not (Variables|Default|GetisJumping))
      (Sprite|SetFlipbook (Variables|Default|GetPaperFlipbook) "/Game/Assets/Player/Animations/Player_Idle.Player_Idle"))))

(event Input|EnhancedActionEvents|EnhancedInputActionIA_Jump
  (params (ActionValue :type Float%20%28double-precision%29) (ElapsedSeconds :type Float%20%28double-precision%29) (TriggeredSeconds :type Float%20%28double-precision%29) (InputAction :type Input%20Action%20Object%20Reference :default "/Game/Assets/Player/Blueprints/IA_Jump.IA_Jump")))

(event EventBeginPlay
  (bind _asbp_player_controller (Utilities|Casting|CastToBP_PlayerController (Pawn|GetController)))
  (Input|AddMappingContext (PlayerController|LocalPlayerSubsystems|GetEnhancedInputLocalPlayerSubsystem _asbp_player_controller) "/Game/Assets/Player/Blueprints/IMC_Default.IMC_Default" 0 "(bIgnoreAllPressedKeysUntilRelease=True,bForceImmediately=False)"))

(fn ConstructionScript)